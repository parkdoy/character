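; BP_ShootingHUD is the shooting game's HUD, creating the on-screen widget at BeginPlay and setting game-only input.
; Update functions forward ammo, magazine, HP, armor and an F-key guide's position and visibility to that widget.
; It binds to the local player state's HP and armor dispatchers; the failed-cast retry timer names BindPlayerState instead of BindMyPlayerState.
; BindPlayerState hooks name, kill and death dispatchers to refresh the player list.
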(event EventBeginPlay
  (bind _returnvalue (Game|GetPlayerController 0))
  (bind _returnvalue_2 (UserInterface|CreateWidget "/Game/ShootingGame/Widget/ShootingHUDWidget.ShootingHUDWidget_C"))
  (bind _output_get (Variables|Default|SetHUDWidget _returnvalue_2))
  (UserInterface|Viewport|AddtoViewport _output_get 0)
  (CallFunction|BindMyPlayerState)
  (Input|SetInputModeGameOnly _returnvalue)
  (Variables|/Script/Engine.PlayerController|SetbShowMouseCursor _returnvalue false))

(fn ConstructionScript)

(fn UpdateAmmo
  (params (Ammo :type Integer))
  (Default|SetAmmo (Variables|Default|GetHUDWidget) Ammo))

(fn UpdateMag
  (params (Mag :type Integer))
  (Default|SetMag (Variables|Default|GetHUDWidget) Mag))

(fn UpdateHP
  (params (CurHp :type Float%20%28single-precision%29) (MaxHp :type Float%20%28single-precision%29))
  (Default|SetHp (Variables|Default|GetHUDWidget) CurHp MaxHp))

(fn UpdateGuideF
  (params (WorldLocation :type Vector))
  (Default|SetPositionGuideF (Variables|Default|GetHUDWidget) WorldLocation))

(fn SetVisibilityGuideF
  (params (InVisibility :type ESlateVisibility%20Enum :default "Visible"))
  (Default|SetVisibilityGuideF (Variables|Default|GetHUDWidget) InVisibility))

(fn BindMyPlayerState
  (bind _asbp_shooting_player_state (Utilities|Casting|CastToBP_ShootingPlayerState (Variables|/Script/Engine.Controller|GetPlayerState (Game|GetPlayerController 0)))
    (:then
      (EventDispatchers|BindEventtoEventDispatcherHP _asbp_shooting_player_state (EventDispatchers|CreateEvent :!event UpdateHP))
      (EventDispatchers|BindEventtoEventDispatcherArmor _asbp_shooting_player_state (EventDispatchers|CreateEvent :!event UpdateArmor)))
    (:CastFailed
      (Utilities|Time|SetTimerbyFunctionName 0 "BindPlayerState" 0.1))))

(fn UpdateArmor
  (params (CurArmor :type Float%20%28single-precision%29) (MaxArmor :type Float%20%28single-precision%29))
  (Default|SetArmor (Variables|Default|GetHUDWidget) CurArmor MaxArmor))

(fn EventChangeName
  (params (NewName :type String))
  (CallFunction|UpdatePlayerList))

(fn UpdatePlayerList
  (bind _hudwidget (Variables|Default|GetHUDWidget))
  (Utilities|IsValid _hudwidget
    (:Is%20Valid
      (Default|UpdatePlayerList _hudwidget))
    (:Is%20Not%20Valid
      (Utilities|Time|SetTimerbyFunctionName 0 "UpdatePlayerList" 0.1))))

(fn BindPlayerState
  (params (PlayerState :type BP%20Shooting%20Player%20State%20Object%20Reference))
  (EventDispatchers|BindEventtoEventDispatcherChangeName PlayerState (EventDispatchers|CreateEvent :!event EventChangeName))
  (EventDispatchers|BindEventtoEventDispatcherKill PlayerState (EventDispatchers|CreateEvent :!event EventKill))
  (EventDispatchers|BindEventtoEventDispatcherDeath PlayerState (EventDispatchers|CreateEvent :!event EventDeath))
  (CallFunction|UpdatePlayerList))

(fn EventKill
  (params (Kill :type Integer))
  (CallFunction|UpdatePlayerList))

(fn EventDeath
  (params (Death :type Integer))
  (CallFunction|UpdatePlayerList))